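; Enemy character that moves toward the player via a single AI MoveTo on BeginPlay and takes damage until its clamped health reaches zero.
; Non-lethal hits play sound, montage and effect, briefly disabling movement before walking resumes.
; Death stops movement, plays sound, montage and a delayed effect before destroying the actor.
; In parallel, death spawns an ammo drop at a downward line trace's hit location, using a weighted roll set to always succeed.
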(event Game|Damage|EventAnyDamage
  (params (Damage :type Float%20%28single-precision%29) (DamageType :type Damage%20Type%20Object%20Reference) (InstigatedBy :type Controller%20Object%20Reference) (DamageCauser :type Actor%20Object%20Reference))
  (bind _returnvalue (Transformation|GetActorLocation))
  ;[0.15 0.15 0.15 0.5] Enemy Lose HP
  (if (not (Variables|Default|GetIsDead))
    (bind _output_get (Variables|Default|SetHealth (Math|Float|Clamp(Float) (- (Variables|Default|GetHealth) Damage) 0.0 1e+02)))
    (if (== _output_get 0.0)
      ;[0.15 0.15 0.15 0.5] Enemy Dead
      (Audio|PlaySound2D "/Game/Audio/HumanVocalizations/HumanMaleA/Cues/voice_male_grunt_pain_death_07_Cue.voice_male_grunt_pain_death_07_Cue" 1.0 1.0 0.0 0 0)
      (Pawn|Components|CharacterMovement|DisableMovement (Variables|Character|GetCharacterMovement))
      (Variables|Default|SetIsDead true)
      (Utilities|FlowControl|Sequence
        (:then_0
          (Animation|PlayAnimMontage "/Game/EnemyAi/Death.Death" 1.0 "None")
          (Utilities|FlowControl|Delay 1.2)
          (Components|Activation|Activate (Variables|Default|GetDeath_Effect) false)
          (Utilities|FlowControl|Delay 1.0)
          (Actor|DestroyActor))
        (:then_1
          ;[0.15 0.15 0.15 0.5] Spawn Ammo
          (if (Math|Random|RandomBoolwithWeight 1.0)
            (bind _outhit (Collision|LineTraceByChannel _returnvalue (- _returnvalue "0.000000,0.000000,1500.000000") "TraceTypeQuery1" false 0 "None"))
            (Game|SpawnActorfromClass "/Game/EnemyAi/BP_AmmoDrop.BP_AmmoDrop_C" (Math|Transform|MakeTransform (.Location (Collision|BreakHitResult _outhit)) "0, 0, 0" "1.000000,1.000000,1.000000") "Undefined" "MultiplyWithRoot" 0 0))))
      (else
        ;[0.15 0.15 0.15 0.5] Enemy Hit
        (Audio|PlaySound2D "/Game/Audio/Bullet_Imapct.Bullet_Imapct" 1.0 1.0 0.0 0 0)
        (Utilities|FlowControl|Sequence
          (:then_0
            (bind _returnvalue_2 (Animation|PlayAnimMontage "/Game/EnemyAi/Hit.Hit" 1.0 "None"))
            (Utilities|FlowControl|Delay _returnvalue_2)
            (if (not (Variables|Default|GetIsDead))
              (Animation|PlayAnimMontage "/Game/EnemyAi/Walking.Walking" 1.0 "None" :!label _label)))
          (:then_1
            (Pawn|Components|CharacterMovement|DisableMovement (Variables|Character|GetCharacterMovement))
            (Utilities|FlowControl|Sequence
              (:then_0
                (Utilities|FlowControl|Delay 0.2)
                (Pawn|Components|CharacterMovement|SetMovementMode (Variables|Character|GetCharacterMovement) "MOVE_Walking" 0)
                (goto _label))
              (:then_1
                (Components|Activation|Activate (Variables|Default|GetNS_Hit_Effect) false)))))))))

(event EventBeginPlay
  ;[0.15 0.15 0.15 0.5] Walks Towards Player
  (Utilities|FlowControl|Sequence
    (:then_0
      (AI|AIMoveTo self "0, 0, 0" (Game|GetPlayerCharacter 0) 5.0 false
        (:then
          (Utilities|FlowControl|Delay 0.2))))))

(fn ConstructionScript)